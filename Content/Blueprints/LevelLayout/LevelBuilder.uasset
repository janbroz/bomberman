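; LevelBuilder generates a grid arena with a pillar at every odd-odd cell, a raised border wall and randomly scattered obstacles.
; The construction script lays centered floor and pillar instanced meshes from Width, Heigth and Size, re-adding the wall on each outer-loop pass.
; It randomly picks floor cells in scan order, capped by the DestructibleBlocks fraction, and stores them in SpawnInfo, which BeginPlay uses to spawn ObstacleClass actors.
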(event EventBeginPlay
  (for _array_element (Variables|Default|GetSpawnInfo)
    (Game|SpawnActorfromClass (Variables|Default|GetObstacleClass) (Utilities|Struct|BreakSpawnData _array_element) "Undefined" 0 0)))

(fn ConstructionScript
  (bind _size (Variables|Default|GetSize))
  (bind _width (Variables|Default|GetWidth))
  (bind _heigth (Variables|Default|GetHeigth))
  (bind _size_2 (Variables|Default|GetSize))
  (bind _width_2 (Variables|Default|GetWidth))
  (bind _heigth_2 (Variables|Default|GetHeigth))
  (bind _size_3 (Variables|Default|GetSize))
  (bind _returnvalue (- _width 1))
  (bind _returnvalue_2 (- _heigth 1))
  (bind _returnvalue_3 (+ _width_2 1))
  (bind _returnvalue_4 (+ _heigth_2 1))
  (bind _returnvalue_5 (Math|Conversions|ToFloat(Integer) _returnvalue_3))
  (bind _returnvalue_6 (Math|Conversions|ToFloat(Integer) _returnvalue_4))
  (bind _returnvalue_7 (/ _returnvalue_5 2.0))
  (bind _returnvalue_8 (/ _returnvalue_6 2.0))
  (Variables|Default|SetPillars 0)
  (bind _output_get (Variables|Default|SetLevelSize (* (Variables|Default|GetWidth) (Variables|Default|GetHeigth))))
  (Variables|Default|SetBlocksToSpawn (Math|Float|Truncate (* _output_get (Variables|Default|GetDestructibleBlocks%25))))
  (Variables|Default|SetBlocksSpawned 0)
  (Utilities|Array|Clear (Variables|Default|GetSpawnInfo))
  ;[1 1 1] Build the floor
  (for _index (range 0 _returnvalue)
    (for _index_2 (range 0 _returnvalue_2)
      (if (> (Class|KismetMathLibrary|AndIntInt (Class|KismetMathLibrary|AndIntInt _index 1) (Class|KismetMathLibrary|AndIntInt _index_2 1)) 0)
        (Components|InstancedStaticMesh|AddInstance (Variables|Default|GetInstancedStaticMeshPilar) (Math|Transform|MakeTransform (Math|Vector|MakeVector (* (- (Math|Conversions|ToFloat(Integer) _index) (/ (Math|Conversions|ToFloat(Integer) _returnvalue) 2.0)) _size_2) (* (- (Math|Conversions|ToFloat(Integer) _index_2) (/ (Math|Conversions|ToFloat(Integer) _returnvalue_2) 2.0)) _size_2) 0.0) "0, 0, 0" "1.000000,1.000000,1.000000"))
        (Math|Integer|IncrementInt (Variables|Default|GetPillars))
        (else
          (if (> (Variables|Default|GetBlocksToSpawn) 0)
            (if (> (Math|Random|RandomInteger 10) 6)
              (Math|Integer|DecrementInt (Variables|Default|GetBlocksToSpawn)
                (:%20%20
                  (Utilities|Array|Add (Variables|Default|GetSpawnInfo) (Utilities|Struct|MakeSpawnData (Math|Transform|MakeTransform (Math|Vector|MakeVector (* (- (Math|Conversions|ToFloat(Integer) _index) (/ (Math|Conversions|ToFloat(Integer) _returnvalue) 2.0)) _size_2) (* (- (Math|Conversions|ToFloat(Integer) _index_2) (/ (Math|Conversions|ToFloat(Integer) _returnvalue_2) 2.0)) _size_2) 0.0) "0, 0, 0" "1.000000,1.000000,1.000000")))))))
          (Components|InstancedStaticMesh|AddInstance (Variables|Default|GetInstancedStaticMeshFloor) (Math|Transform|MakeTransform (Math|Vector|MakeVector (* (- (Math|Conversions|ToFloat(Integer) _index) (/ (Math|Conversions|ToFloat(Integer) _returnvalue) 2.0)) _size_2) (* (- (Math|Conversions|ToFloat(Integer) _index_2) (/ (Math|Conversions|ToFloat(Integer) _returnvalue_2) 2.0)) _size_2) 0.0) "0, 0, 0" "1.000000,1.000000,1.000000")))))
    ;[1 1 1] Build the wall
    (for _index_3 (range 0 _returnvalue_3)
      (for _array_element (LocalVariables|GetNegAndPos)
        (Components|InstancedStaticMesh|AddInstance (Variables|Default|GetInstancedStaticMeshPilar) (Math|Transform|MakeTransform (Math|Vector|MakeVector (* (- (Math|Conversions|ToFloat(Integer) _index_3) _returnvalue_7) _size_3) (* _array_element (* _returnvalue_8 _size_3)) 0.0) "0, 0, 0" "1.000000,1.000000,1.500000"))))
    (for _index_4 (range 0 _returnvalue_4)
      (for _array_element_2 (LocalVariables|GetNegAndPos)
        (Components|InstancedStaticMesh|AddInstance (Variables|Default|GetInstancedStaticMeshPilar) (Math|Transform|MakeTransform (Math|Vector|MakeVector (* _array_element_2 (* _returnvalue_7 _size)) (* (- (Math|Conversions|ToFloat(Integer) _index_4) _returnvalue_8) _size) 0.0) "0, 0, 0" "1.000000,1,1.500000"))))))